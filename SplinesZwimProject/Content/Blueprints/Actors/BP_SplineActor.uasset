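; BP_SplineActor is a construction-script tool that repeats a chosen static mesh along a spline.
; It derives section length from the mesh bounds (extent minus origin) on the selected forward axis, plus a spacing value.
; At each interval it adds a spline mesh component at the spline's location and rotation, combined with a rotation offset.
; Start/end points and tangents are never set, so segments do not bend to follow the curve.
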(event EventBeginPlay)

(event Collision|EventActorBeginOverlap
  (params (OtherActor :type Actor%20Object%20Reference)))

(event EventTick
  (params (DeltaSeconds :type Float%20%28single-precision%29)))

(fn ConstructionScript
  (bind _spline_mesh (Variables|Default|GetSpline%20Mesh))
  (bind _spline (Variables|Default|GetSpline))
  (bind _returnvalue (StaticMesh|GetBounds _spline_mesh))
  (bind _returnvalue_2 (- (.boxextent _returnvalue) (.origin _returnvalue)))
  (Utilities|IsValid (Variables|Default|GetSpline%20Mesh)
    (:Is%20Valid
      (switch Utilities|FlowControl|Switch|SwitchonESplineMeshAxis (Variables|Default|GetIn%20Forward%20Axis)
        (:X
          (Variables|Default|SetMesh%20Length (.x _returnvalue_2)))
        (:Y
          (Variables|Default|SetMesh%20Length (.y _returnvalue_2)))
        (:Z
          (Variables|Default|SetMesh%20Length (.z _returnvalue_2))))
      (Variables|Default|SetSectionLength (+ (Variables|Default|GetSpacing) (Variables|Default|GetMesh%20Length)))
      (for _index (range 0 (Math|Float|Truncate (/ (Spline|GetSplineLength (Variables|Default|GetSpline)) (Variables|Default|GetSectionLength))))
        (Variables|Default|SetIndex _index)
        (bind _returnvalue_3 (AddComponent|AddSplineMeshComponent false (Math|Transform|MakeTransform (Spline|GetLocationatDistanceAlongSpline _spline (* (Variables|Default|GetIndex) (Variables|Default|GetSectionLength)) "Local") (Math|Rotator|CombineRotators (Variables|Default|GetMeshRotation) (Spline|GetRotationatDistanceAlongSpline _spline (* (Variables|Default|GetIndex) (Variables|Default|GetSectionLength)) "Local")))))
        (Components|StaticMesh|SetStaticMesh _returnvalue_3 (Variables|Default|GetSpline%20Mesh))
        (SplineMesh|SetForwardAxis _returnvalue_3 (Variables|Default|GetIn%20Forward%20Axis) true)))))